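; BP_StorageMobile is a temporary actor that presents a 3D storage inventory with an animated skeletal mesh and its own camera view.
; On BeginPlay it plays the opening animation, blends the player's view to itself and initializes its 3D inventory component.
; CE_CloseInventory plays the animation in reverse, then deinitializes the inventory and destroys the actor after a short delay.
; LinkInventory points the 3D inventory component at an inventory component.
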(event LinkInventory(AC_3DInventory)
  (Variables|/Game/Inventory3D/Blueprints/AC_3DInventory.AC_3DInventory_C|SetInventoryRef (Variables|Default|GetAC_3DInventory) (Variables|Default|GetAC_Inventory)))

(event Custom|CE_CloseInventory
  (Components|Timeline|SetPlayRate (Variables|Default|GetSkeletalMesh) -1.0)
  (Components|Animation|SetPosition (Variables|Default|GetSkeletalMesh) 0.6 false)
  (Audio|Components|Audio|Play (Variables|Default|GetSkeletalMesh) false)
  (Utilities|FlowControl|Delay 0.6)
  (Default|Deinitialize (Variables|Default|GetAC_3DInventory))
  (Actor|DestroyActor))

(event EventBeginPlay
  (Audio|Components|Audio|Play (Variables|Default|GetSkeletalMesh) false)
  (Game|Player|SetViewTargetwithBlend (Game|GetPlayerController 0) self 0.6 "VTBlend_Linear" 0.0 false)
  (Default|Initialize (Variables|Default|GetAC_3DInventory)))

(event Collision|EventActorBeginOverlap
  (params (OtherActor :type Actor%20Object%20Reference)))

(event EventTick
  (params (DeltaSeconds :type Float%20%28single-precision%29)))

(fn ConstructionScript)