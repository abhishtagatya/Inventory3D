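; Actor component that presents an inventory in 3D, pairing a UMG slot grid with spawned item actors.
; Initialize finds the owner's grid widget and inventory, calls LinkInventory if the inventory is missing, and destroys itself if requirements are unmet.
; Populate sizes the grid and attaches an actor per entry to the widget component, passing its data.
; It relays slot hovers through dispatchers and mirrors item adds and removals to the inventory.
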(event EventBeginPlay)

(event EventTick
  (params (DeltaSeconds :type Float%20%28single-precision%29)))

(fn ReceiveHoverExitSlot
  (params (Slot :type UMG%20Slot%20Object%20Reference))
  (Default|CallHoverExitSlot self Slot))

(fn ReceiveHoverSlot
  (params (Slot :type UMG%20Slot%20Object%20Reference))
  (Default|CallHoverSlot self Slot))

(fn Deinitialize
  (for _array_element (Variables|Inventory|GetItems)
    (Actor|DestroyActor _array_element)))

(fn Populate
  (bind _inventoryref (Variables|Inventory|GetInventoryRef))
  (Default|CreateEmptyGrid (Variables|Widget|GetUMG_Grid) (Variables|/Game/Inventory3D/Blueprints/AC_Inventory.AC_Inventory_C|GetTotalSlots _inventoryref) (Variables|/Game/Inventory3D/Blueprints/AC_Inventory.AC_Inventory_C|GetColumns _inventoryref))
  (for _array_element (Variables|/Game/Inventory3D/Blueprints/AC_Inventory.AC_Inventory_C|GetInventory (Variables|Inventory|GetInventoryRef))
    (bind _returnvalue (Game|SpawnActorfromClass (Variables|Inventory|GetItemClass) (Math|Transform|MakeTransform "0, 0, 0") "Undefined" "MultiplyWithRoot" (Components|GetOwner) 0))
    (Class|BPIShareInfo|SetTotalData(Message) _returnvalue _array_element)
    (Utilities|Array|Add (Variables|Inventory|GetItems) _returnvalue)
    (Transformation|AttachComponentToComponent _returnvalue (Variables|Widget|GetWidgetComp) "None" "KeepRelative" "KeepRelative" "KeepRelative" false)))

(fn Initialize
  (bind _returnvalue (Components|GetOwner))
  (bind _returnvalue_2 (Components|GetOwner))
  (bind _returnvalue_3 (Actor|GetComponentbyClass _returnvalue "/Script/UMG.WidgetComponent"))
  (bind _returnvalue_4 (Actor|GetComponentbyClass _returnvalue_2 "/Game/Inventory3D/Blueprints/AC_Inventory.AC_Inventory_C"))
  (Utilities|FlowControl|Sequence
    (:then_0
      (Utilities|IsValid _returnvalue_3
        (:Is%20Valid
          (bind _output_get (Variables|Widget|SetWidgetComp _returnvalue_3))
          (bind _asumg_grid (Utilities|Casting|CastToUMG_Grid (UserInterface|GetWidget _output_get)))
          (Variables|Widget|SetUMG_Grid _asumg_grid)
          (EventDispatchers|BindEventtoGridSlotHover (Variables|Widget|GetUMG_Grid) (EventDispatchers|CreateEvent :!event ReceiveHoverSlot))
          (EventDispatchers|BindEventtoGridSlotHoverExit (Variables|Widget|GetUMG_Grid) (EventDispatchers|CreateEvent :!event ReceiveHoverExitSlot)))))
    (:then_1
      (Utilities|IsValid _returnvalue_4
        (:Is%20Valid
          (Variables|Inventory|SetInventoryRef _returnvalue_4))
        (:Is%20Not%20Valid
          (Default|CallLinkInventory)))
      (if (Math|Boolean|ANDBoolean (Utilities|IsValid (Variables|Widget|GetUMG_Grid)) (Utilities|IsValid (Variables|Inventory|GetInventoryRef)) (Class|KismetSystemLibrary|DoesClassImplementInterface (Variables|Inventory|GetItemClass) "/Game/Inventory3D/Blueprints/BPI_ShareInfo.BPI_ShareInfo_C"))
        (Constructor|Populate)
        (else
          (Components|DestroyComponent))))))

(fn RemoveItemfromInventory
  (params (Item :type Actor%20Object%20Reference))
  (Default|RemoveItemfromInventory (Variables|Inventory|GetInventoryRef) (Default|GetCompleteData (Variables|Inventory|GetInventoryRef) Item))
  (Utilities|Array|RemoveItem (Variables|Inventory|GetItems) Item))

(fn AddItemtoInventory
  (params (Item :type Actor%20Object%20Reference))
  (Default|AddItemtoInventory (Variables|Inventory|GetInventoryRef) (Default|GetCompleteData (Variables|Inventory|GetInventoryRef) Item))
  (Utilities|Array|Add (Variables|Inventory|GetItems) Item))