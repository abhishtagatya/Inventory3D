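; Inventory component that stores shaped, stackable items on a slot grid, tracking occupied coordinates in a map and filling prepopulated items at BeginPlay.
; Adding an item tops up matching partial stacks, then scans for free space, trying the priority rotation before the other right angles.
; ItemInteract builds item data through BPI_ShareInfo and writes any remaining quantity back when the item doesn't fit.
; Helpers handle removal and finding stackable items overlapping given coordinates.
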(event EventBeginPlay
  (Setup|InitializeOccupiedSlots)
  (Variables|Setup|SetItemRotationPriority (|EnsureValidRotation)))

(event EventTick
  (params (DeltaSeconds :type Float%20%28single-precision%29)))

(fn TryAddItem
  (params (Item :type ST%20Inventory%20Item%20Structure))
  (LocalVariables|SetLItemInfo Item)
  (Utilities|FlowControl|Sequence
    (:then_0
      (bind (_found _item) (Conditions|DoesContainItem (.ObjectRef (Utilities|Struct|BreakST_InventoryItem (LocalVariables|GetLItemInfo)))))
      (if _found
        (for _array_element _item
          (AddItem|AddQuantitytoSlot _array_element (.Quantity (Utilities|Struct|BreakST_InventoryItem (LocalVariables|GetLItemInfo))))
          (if (<= (.Quantity (Utilities|Struct|BreakST_InventoryItem (LocalVariables|GetLItemInfo))) 0)
            (return true 0)))))
    (:then_1
      (bind _slot (Utilities|ForEachSlot (Variables|Setup|GetTotalSlots) (Variables|Setup|GetColumns))
        (:Loop%20Body
          (bind (_doesfit _rotationused) (Conditions|CanAddtoSlot _slot (Utilities|Struct|BreakST_InventoryItem (LocalVariables|GetLItemInfo))))
          (if _doesfit
            (bind _structout (Utilities|Struct|SetmembersinST_InventoryItem (LocalVariables|GetLItemInfo) _slot _rotationused))
            (Direct|AddItemtoInventory _structout)
            (return true 0)))
        (:Completed
          (return false (Utilities|Struct|BreakST_InventoryItem (LocalVariables|GetLItemInfo))))))))

(fn ItemInteract
  (params (Input :type Actor%20Object%20Reference%20%28by%20ref%29))
  (if (Utilities|DoesObjectImplementInterface Input "/Game/Inventory3D/Blueprints/BPI_ShareInfo.BPI_ShareInfo_C")
    (bind (_destroyitem _remaining) (AddItem|TryAddItem (Getters|GetCompleteData Input)))
    (if _destroyitem
      (return true)
      (else
        (Class|BPIShareInfo|SetQuantity(Message) Input _remaining)
        (return false)))
    (else
      (return false))))

(fn AddQuantitytoSlot
  (params (Input :type ST%20Inventory%20Item%20Structure) (Quantity :type Integer%20%28by%20ref%29))
  (bind _output_get (LocalVariables|SetLNewStructure Input))
  (LocalVariables|SetLNewQuantity (Math|Integer|Clamp(Integer) (+ (.Quantity (Utilities|Struct|BreakST_InventoryItem _output_get)) Quantity) 1 (.MaxQuantity (Utilities|Struct|BreakST_InventoryItem _output_get))))
  (|SetBy-RefVar Quantity (- (+ (.Quantity (Utilities|Struct|BreakST_InventoryItem (LocalVariables|GetLNewStructure))) Quantity) (.MaxQuantity (Utilities|Struct|BreakST_InventoryItem (LocalVariables|GetLNewStructure)))))
  (Utilities|Struct|SetmembersinST_InventoryItem (LocalVariables|GetLNewStructure) (LocalVariables|GetLNewQuantity))
  (Utilities|Array|SetArrayElem (Variables|Storage|GetInventory) (Utilities|Array|FindItem (Variables|Storage|GetInventory) Input) (LocalVariables|GetLNewStructure)))

(fn DoesContainItem
  (params (In :type Object%20Soft%20Object%20Reference))
  (bind _llocalitems (LocalVariables|GetLLocalItems))
  (for _array_element (Variables|Storage|GetInventory)
    (if (and (!= (.Quantity (Utilities|Struct|BreakST_InventoryItem _array_element)) (.MaxQuantity (Utilities|Struct|BreakST_InventoryItem _array_element))) (== (.ObjectRef (Utilities|Struct|BreakST_InventoryItem _array_element)) In))
      (Utilities|Array|Add (LocalVariables|GetLLocalItems) _array_element)))
  (return (Utilities|Array|IsNotEmpty _llocalitems) _llocalitems))

(fn CanAddtoSlot
  (params (Coordinates :type Vector%202D%20Structure) (Shape :type Array%20of%20Vector%202D%20Structures))
  (if (Conditions|AreSlotsAvailable (Getters|GetRelevantCoordinates Coordinates Shape (Variables|Setup|GetItemRotationPriority)))
    (return true (Variables|Setup|GetItemRotationPriority))
    (else
      (for _index (range 0 3)
        (Utilities|FlowControl|Sequence
          (:then_0
            (switch int _index
              (:0
                (LocalVariables|SetLTestAngle 0.0))
              (:1
                (LocalVariables|SetLTestAngle 9e+01))
              (:2
                (LocalVariables|SetLTestAngle 1.8e+02))
              (:3
                (LocalVariables|SetLTestAngle -9e+01))))
          (:then_1
            (if (!= (LocalVariables|GetLTestAngle) (Variables|Setup|GetItemRotationPriority))
              (if (Conditions|AreSlotsAvailable (Getters|GetRelevantCoordinates Coordinates Shape (LocalVariables|GetLTestAngle)))
                (return true (LocalVariables|GetLTestAngle)))))))
      (return false 0.0))))

(fn AreSlotsAvailable
  (params (InputPin :type Array%20of%20Vector%202D%20Structures) (Ignore :type Array%20of%20Vector%202D%20Structures))
  (for _array_element InputPin
    (if (not (Utilities|Array|ContainsItem Ignore _array_element))
      (if (.ReturnValue (Utilities|Map|Find (Variables|Storage|GetOccupiedSlots) _array_element))
        (if (.Value (Utilities|Map|Find (Variables|Storage|GetOccupiedSlots) _array_element))
          (return false))
        (else
          (return false)))))
  (return true))

(fn RemoveItemfromInventory
  (params (NewItem :type ST%20Inventory%20Item%20Structure))
  (bind _output_get (LocalVariables|SetLData NewItem))
  (bind _output_get_2 (LocalVariables|SetLRelevantShape (Getters|GetRelevantCoordinates (.Coordinates (Utilities|Struct|BreakST_InventoryItem _output_get)) (.ItemShape (Utilities|Struct|BreakST_InventoryItem _output_get)) (.ItemRotation (Utilities|Struct|BreakST_InventoryItem _output_get)))))
  (for _array_element _output_get_2
    (Utilities|Map|Add (Variables|Storage|GetOccupiedSlots) _array_element false))
  (Utilities|Array|RemoveItem (Variables|Storage|GetInventory) NewItem))

(fn AddItemtoInventory
  (params (NewItem :type ST%20Inventory%20Item%20Structure))
  (bind _output_get (LocalVariables|SetLData NewItem))
  (bind _output_get_2 (LocalVariables|SetLRelevantShape (Getters|GetRelevantCoordinates (.Coordinates (Utilities|Struct|BreakST_InventoryItem _output_get)) (.ItemShape (Utilities|Struct|BreakST_InventoryItem _output_get)) (.ItemRotation (Utilities|Struct|BreakST_InventoryItem _output_get)))))
  (for _array_element _output_get_2
    (Utilities|Map|Add (Variables|Storage|GetOccupiedSlots) _array_element true))
  (Utilities|Array|Add (Variables|Storage|GetInventory) NewItem))

(fn InitializeOccupiedSlots
  (bind _slot (Utilities|ForEachSlot (Variables|Setup|GetTotalSlots) (Variables|Setup|GetColumns))
    (:Loop%20Body
      (Utilities|Map|Add (Variables|Storage|GetOccupiedSlots) _slot false))
    (:Completed
      (for _array_element (Variables|Storage|GetPrepoulation)
        (bind _structout (Utilities|Struct|SetmembersinST_InventoryItem (Getters|GetCompleteData (.DataAsset (Utilities|Struct|BreakST_Prepopulate _array_element))) (Math|Integer|Clamp(Integer) (.Quantity (Utilities|Struct|BreakST_Prepopulate _array_element)) 1 (Utilities|Struct|BreakST_InventoryItem (Getters|GetCompleteData (.DataAsset (Utilities|Struct|BreakST_Prepopulate _array_element)))))))
        (AddItem|TryAddItem _structout)))))

(fn GetRelevantCoordinates
  (params (Coordinates :type Vector%202D%20Structure) (Shape :type Array%20of%20Vector%202D%20Structures) (Rotation :type Float%20%28double-precision%29))
  (bind _rotatedshape (Utilities|Rotate2DArray Shape Rotation)
    (:%20%20
      (bind _output_get (LocalVariables|SetLRotatedShape _rotatedshape))
      (for (_array_element _array_index) _output_get
        (Utilities|Array|SetArrayElem (LocalVariables|GetLRotatedShape) _array_index (+ _array_element Coordinates)))
      (return (LocalVariables|GetLRotatedShape)))))

(fn GetRelevantItems
  (params (Coordinates :type Array%20of%20Vector%202D%20Structures) (Object :type Object%20Soft%20Object%20Reference))
  (Utilities|Set|AddItems (LocalVariables|GetLInputCoords) Coordinates)
  (for (_array_element _array_index) (Variables|Storage|GetInventory)
    (LocalVariables|SetLCurrentItem _array_element)
    (LocalVariables|SetLCurrentIndex _array_index)
    (Utilities|Set|Clear (LocalVariables|GetLCurrentItemSet))
    (Utilities|Set|AddItems (LocalVariables|GetLCurrentItemSet) (Getters|GetRelevantCoordinates (.Coordinates (Utilities|Struct|BreakST_InventoryItem (LocalVariables|GetLCurrentItem))) (.ItemShape (Utilities|Struct|BreakST_InventoryItem (LocalVariables|GetLCurrentItem))) (.ItemRotation (Utilities|Struct|BreakST_InventoryItem (LocalVariables|GetLCurrentItem)))))
    (bind _result (Utilities|Set|Intersection (LocalVariables|GetLInputCoords) (LocalVariables|GetLCurrentItemSet)))
    (if (Utilities|Set|IsNotEmpty _result)
      (if (== (Utilities|Struct|BreakST_InventoryItem (LocalVariables|GetLCurrentItem)) Object)
        (if (!= (.Quantity (Utilities|Struct|BreakST_InventoryItem (LocalVariables|GetLCurrentItem))) (.MaxQuantity (Utilities|Struct|BreakST_InventoryItem (LocalVariables|GetLCurrentItem))))
          (Utilities|Array|Add (LocalVariables|GetLReturnArray) (LocalVariables|GetLCurrentIndex))))))
  (return (LocalVariables|GetLReturnArray)))

(fn GetCompleteData
  (params (Input :type Object%20Object%20Reference))
  (bind _coordinates (Class|BPIShareInfo|GetCoordinates(Message) Input))
  (bind _quantity (Class|BPIShareInfo|GetQuantity(Message) Input))
  (bind _quantity_2 (Class|BPIShareInfo|GetMaxQuantity(Message) Input))
  (bind _itemname (Class|BPIShareInfo|GetItemName(Message) Input))
  (bind _itemmodel (Class|BPIShareInfo|GetItemModel(Message) Input))
  (bind _itemshape (Class|BPIShareInfo|GetItemShape(Message) Input))
  (bind _itemrotation (Class|BPIShareInfo|GetItemRotation(Message) Input))
  (bind _objectref (Class|BPIShareInfo|GetObjectRef(Message) Input))
  (return (Utilities|Struct|MakeST_InventoryItem _coordinates _quantity _quantity_2 _itemname _itemmodel _itemshape _itemrotation _objectref)))