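; Actor component that lets its owner pick up nearby items into its AC_Inventory component.
; It tracks overlapping items and each tick shows a prompt widget at the closest one's location with its name and quantity.
; The pickup input plays a grab montage, whose "Take Item" notify passes the closest item to the inventory.
; If the inventory accepts it, the item leaves the overlap list and is destroyed.
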(event Custom|EndOverlap
  (params (Target :type Actor%20Object%20Reference))
  (if (Utilities|Array|ContainsItem (Variables|Default|GetOverlappingActors) Target)
    (CallFunction|RemovefromInteraction Target)
    (Widget|SetVisibility (Variables|Default|GetUMG_InteractRef) "Hidden")))

(event Custom|BeginOverlap
  (params (Target :type Actor%20Object%20Reference))
  (Utilities|Array|Add (Variables|Default|GetOverlappingActors) Target)
  (Widget|SetVisibility (Variables|Default|GetUMG_InteractRef) "SelfHitTestInvisible"))

(event Input|EnhancedActionEvents|EnhancedInputActionIA_PickUp
  (params (ActionValue :type Boolean) (ElapsedSeconds :type Float%20%28double-precision%29) (TriggeredSeconds :type Float%20%28double-precision%29) (InputAction :type Input%20Action%20Object%20Reference :default "/Game/Inventory3D/Inputs/IA_PickUp.IA_PickUp"))
  (bind _returnvalue (Components|GetOwner))
  (bind _returnvalue_2 (Actor|GetComponentbyClass _returnvalue "/Script/Engine.SkeletalMeshComponent"))
  (if (Utilities|Array|IsNotEmpty (Variables|Default|GetOverlappingActors))
    (Utilities|IsValid _returnvalue_2
      (:Is%20Valid
        (bind _notifyname (Animation|Montage|PlayMontage _returnvalue_2 "/Game/Inventory3D/Assets/3D_Items/N_Grab_Anim_Montage.N_Grab_Anim_Montage")
          (:OnNotifyBegin
            (switch name _notifyname
              (:TakeItem
                (CallFunction|TryPickupItem)))))))))

(event EventBeginPlay
  (bind _returnvalue (Game|GetPlayerController 0))
  (bind _returnvalue_2 (Components|GetOwner))
  (bind _returnvalue_3 (Actor|GetComponentbyClass _returnvalue_2 "/Game/Inventory3D/Blueprints/AC_Inventory.AC_Inventory_C"))
  (Utilities|IsValid _returnvalue
    (:Is%20Valid
      (Input|AddMappingContext (PlayerController|LocalPlayerSubsystems|GetEnhancedInputLocalPlayerSubsystem _returnvalue) "/Game/Inventory3D/Inputs/IMC_Interact.IMC_Interact" 0 "(bIgnoreAllPressedKeysUntilRelease=True,bForceImmediately=False,bNotifyUserSettings=False)")
      (bind _returnvalue_4 (UserInterface|CreateWidget "/Game/Inventory3D/Widgets/UMG_Interact.UMG_Interact_C"))
      (bind _output_get (Variables|Default|SetUMG_InteractRef _returnvalue_4))
      (UserInterface|Viewport|AddtoViewport _output_get 0)
      (Widget|SetVisibility (Variables|Default|GetUMG_InteractRef) "Hidden")
      (Utilities|IsValid _returnvalue_3
        (:Is%20Valid
          (Variables|Default|SetAC%20Inventory%20Ref _returnvalue_3))))))

(event EventTick
  (params (DeltaSeconds :type Float%20%28single-precision%29))
  (CallFunction|UpdateInteractText))

(fn RemovefromInteraction
  (params (Actor :type Actor%20Object%20Reference))
  (Utilities|Array|RemoveItem (Variables|Default|GetOverlappingActors) Actor)
  (if (Utilities|Array|IsEmpty (Variables|Default|GetOverlappingActors))
    (Widget|SetVisibility (Variables|Default|GetUMG_InteractRef) "Hidden")))

(fn UpdateInteractText
  (bind _umg_interactref (Variables|Default|GetUMG_InteractRef))
  (if (Utilities|Array|IsNotEmpty (Variables|Default|GetOverlappingActors))
    (bind _output_get (LocalVariables|SetLActor (CallFunction|GetClosestActor)))
    (Variables|/Game/Inventory3D/Widgets/UMG_Interact.UMG_Interact_C|SetWorldLocation _umg_interactref (Transformation|GetActorLocation _output_get))
    (bind _itemname (Class|BPIShareInfo|GetItemName(Message) (LocalVariables|GetLActor)))
    (bind _quantity (Class|BPIShareInfo|GetQuantity(Message) (LocalVariables|GetLActor)))
    (Default|UpdateText _umg_interactref _itemname _quantity)))

(fn GetClosestActor
  (for _array_element (Variables|Default|GetOverlappingActors)
    (bind _output_get (LocalVariables|SetLCurrentActor _array_element))
    (LocalVariables|SetLCurrentDistance (Math|Vector|Distance(Vector) (Transformation|GetActorLocation _output_get) (Transformation|GetActorLocation (Components|GetOwner))))
    (if (or (<= (LocalVariables|GetLCurrentDistance) (LocalVariables|GetLMaxDistance)) (== (LocalVariables|GetLMaxDistance) -1.0))
      (LocalVariables|SetLMaxDistance (LocalVariables|GetLCurrentDistance))
      (LocalVariables|SetLReturnActor (LocalVariables|GetLCurrentActor))))
  (return (LocalVariables|GetLReturnActor)))

(fn TryPickupItem
  (Variables|Default|GetAC%20Inventory%20Ref
    (:then
      (LocalVariables|SetLClosestItem (CallFunction|GetClosestActor))
      (bind _candestroyitem (Default|ItemInteract (Variables|Default|GetAC%20Inventory%20Ref) (LocalVariables|GetLClosestItem)))
      (if _candestroyitem
        (CallFunction|RemovefromInteraction (LocalVariables|GetLClosestItem))
        (Actor|DestroyActor (LocalVariables|GetLClosestItem))))
    (:else)))