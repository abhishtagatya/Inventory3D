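; Item actor for a grid-based 3D inventory that exists either as a world pickup or inside an inventory.
; Holds an item data struct, filled from a prepopulated data asset when ownerless, and alerts overlapping interact components.
; Responds to drag, rotate, reset and merge events from a bound handler.
; Uses the rotated item shape and grab point to align the mesh and quantity text to grid cells.
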(event OnComponentBeginOverlap(Sphere)
  (params (OverlappedComponent :type Primitive%20Component%20Object%20Reference) (OtherActor :type Actor%20Object%20Reference) (OtherComp :type Primitive%20Component%20Object%20Reference) (OtherBodyIndex :type Integer) (bFromSweep :type Boolean) (SweepResult :type Hit%20Result%20Structure%20%28by%20ref%29))
  (bind _returnvalue (Actor|GetComponentbyClass OtherActor "/Game/Inventory3D/Blueprints/AC_Interact.AC_Interact_C"))
  (Utilities|IsValid _returnvalue
    (:Is%20Valid
      (Utilities|IsValid (Components|GetOwner)
        (:Is%20Not%20Valid
          (Default|BeginOverlap _returnvalue self))))))

(event OnComponentEndOverlap(Sphere)
  (params (OverlappedComponent :type Primitive%20Component%20Object%20Reference) (OtherActor :type Actor%20Object%20Reference) (OtherComp :type Primitive%20Component%20Object%20Reference) (OtherBodyIndex :type Integer))
  (bind _returnvalue (Actor|GetComponentbyClass OtherActor "/Game/Inventory3D/Blueprints/AC_Interact.AC_Interact_C"))
  (Utilities|IsValid _returnvalue
    (:Is%20Valid
      (Utilities|IsValid (Components|GetOwner)
        (:Is%20Not%20Valid
          (Default|EndOverlap _returnvalue self))))))

(event EventBeginPlay
  (Utilities|IsValid (Components|GetOwner)
    (:Is%20Not%20Valid
      (Development|SetHiddeninGame (Variables|Default|GetTextRender) true false)
      (|ConvertPre-Populated))))

(event Collision|EventActorBeginOverlap
  (params (OtherActor :type Actor%20Object%20Reference)))

(event EventTick
  (params (DeltaSeconds :type Float%20%28single-precision%29)))

(event EventSetTotalData
  (params (NewData :type ST%20Inventory%20Item%20Structure))
  (Variables|Default|SetItemData NewData)
  (Components|StaticMesh|SetStaticMesh (Variables|Default|GetStaticMesh) (Utilities|Struct|BreakST_InventoryItem (Variables|Default|GetItemData)))
  (bind _itemrotation (CallFunction|GetItemRotation))
  (Variables|Default|SetCurrentRotation _itemrotation)
  (EventDispatcher|Local|ReceiveDragEnterInventory)
  (Transform|AdjustRotation)
  (Text|ModifyTextQuantity)
  (Transform|AdjustLocation))

(event EventBindEventHandler
  (params (Handler :type AC%20Handler%20Object%20Reference))
  (EventDispatchers|BindEventtoDragHoverInventory Handler (EventDispatchers|CreateEvent :!event ReceiveDragEnterInventory))
  (EventDispatchers|BindEventtoDragHoverExitInventory Handler (EventDispatchers|CreateEvent :!event ReceiveDragExitInventory))
  (EventDispatchers|BindEventtoStartDragWorld Handler (EventDispatchers|CreateEvent :!event ReceiveStartDragWorld))
  (EventDispatchers|BindEventtoStartDragInventory Handler (EventDispatchers|CreateEvent :!event ReceiveStartDragInventory))
  (EventDispatchers|BindEventtoEndDragInventory Handler (EventDispatchers|CreateEvent :!event ReceiveEndDragInventory))
  (EventDispatchers|BindEventtoEndDragWorld Handler (EventDispatchers|CreateEvent :!event ReceiveEndDragWorld))
  (EventDispatchers|BindEventtoResetDragInventory Handler (EventDispatchers|CreateEvent :!event ReceiveResetDragInventory))
  (EventDispatchers|BindEventtoResetDragWorld Handler (EventDispatchers|CreateEvent :!event ReceiveResetDragWorld))
  (EventDispatchers|BindEventtoRotateItemInventory Handler (EventDispatchers|CreateEvent :!event ReceiveRotateItemInventory))
  (EventDispatchers|BindEventtoMergeItem Handler (EventDispatchers|CreateEvent :!event ReceiveMergeItemInventory))
  (EventDispatchers|BindEventtoConsumedIteminMerge Handler (EventDispatchers|CreateEvent :!event ReceiveConsumedItemInventory)))

(event EventUnbindEventHandler
  (params (Handler :type AC%20Handler%20Object%20Reference))
  (EventDispatchers|UnbindEventfromDragHoverInventory Handler (EventDispatchers|CreateEvent :!event ReceiveDragEnterInventory))
  (EventDispatchers|UnbindEventfromDragHoverExitInventory Handler (EventDispatchers|CreateEvent :!event ReceiveDragExitInventory))
  (EventDispatchers|UnbindEventfromStartDragWorld Handler (EventDispatchers|CreateEvent :!event ReceiveStartDragWorld))
  (EventDispatchers|UnbindEventfromStartDragInventory Handler (EventDispatchers|CreateEvent :!event ReceiveStartDragInventory))
  (EventDispatchers|UnbindEventfromEndDragInventory Handler (EventDispatchers|CreateEvent :!event ReceiveEndDragInventory))
  (EventDispatchers|UnbindEventfromEndDragWorld Handler (EventDispatchers|CreateEvent :!event ReceiveEndDragWorld))
  (EventDispatchers|UnbindEventfromResetDragInventory Handler (EventDispatchers|CreateEvent :!event ReceiveResetDragInventory))
  (EventDispatchers|UnbindEventfromResetDragWorld Handler (EventDispatchers|CreateEvent :!event ReceiveResetDragWorld))
  (EventDispatchers|UnbindEventfromRotateItemInventory Handler (EventDispatchers|CreateEvent :!event ReceiveRotateItemInventory))
  (EventDispatchers|UnbindEventfromMergeItem Handler (EventDispatchers|CreateEvent :!event ReceiveMergeItemInventory))
  (EventDispatchers|UnbindEventfromConsumedIteminMerge Handler (EventDispatchers|CreateEvent :!event ReceiveConsumedItemInventory)))

(event EventSetCoordinates
  (params (NewCoordinates :type Vector%202D%20Structure))
  (Utilities|Struct|SetmembersinST_InventoryItem (Variables|Default|GetItemData) NewCoordinates))

(event EventSetQuantity
  (params (NewQuantity :type Integer))
  (bind _quantity (CallFunction|GetMaxQuantity))
  (Utilities|Struct|SetmembersinST_InventoryItem (Variables|Default|GetItemData) (Math|Integer|Clamp(Integer) NewQuantity 0 _quantity))
  (Text|ModifyTextQuantity))

(event EventSetRotation
  (params (NewRotation :type Float%20%28double-precision%29))
  (bind _output_get (Variables|Default|SetCurrentRotation NewRotation))
  (Utilities|Struct|SetmembersinST_InventoryItem (Variables|Default|GetItemData) _output_get))

(fn ConstructionScript
  (bind _prepoulatedinfo (Variables|Default|GetPrepoulatedInfo))
  (bind (_quantity _dataasset) (Utilities|Struct|BreakST_Prepopulate _prepoulatedinfo))
  (Utilities|IsValid (Utilities|Struct|BreakST_Prepopulate (Variables|Default|GetPrepoulatedInfo))
    (:Is%20Valid
      (bind _itemmodel (Default|GetItemModel (Utilities|Struct|BreakST_Prepopulate (Variables|Default|GetPrepoulatedInfo))))
      (Components|StaticMesh|SetStaticMesh (Variables|Default|GetStaticMesh) _itemmodel)
      (bind _quantity_2 (Default|GetMaxQuantity _dataasset))
      (Utilities|Struct|SetmembersinST_Prepopulate (Variables|Default|GetPrepoulatedInfo) (Math|Integer|Min(Integer) _quantity_2 _quantity)))))

(fn GetTextCoordinates
  (params (Shape :type Array%20of%20Vector%202D%20Structures) (Position :type E_TextLocation%20Enum :default "NewEnumerator0"))
  (LocalVariables|SetLPosition (Utilities|Select :Index Position :NewEnumerator0 "(X=0.000000,Y=9.000000)" :NewEnumerator1 "(X=9.000000,Y=9.000000)" :NewEnumerator2 "(X=9.000000,Y=0.000000)" :NewEnumerator3 "(X=9.000000,Y=9.000000)"))
  (for _array_element Shape
    (LocalVariables|SetLCurrent _array_element)
    (switch Utilities|FlowControl|Switch|SwitchonE_TextLocation Position
      (:NewEnumerator0
        (if (or (> (.x (LocalVariables|GetLCurrent)) (.x (LocalVariables|GetLPosition))) (< (.y (LocalVariables|GetLCurrent)) (.y (LocalVariables|GetLPosition))))
          (LocalVariables|SetLPosition (LocalVariables|GetLCurrent))))
      (:NewEnumerator1
        (if (or (< (.x (LocalVariables|GetLCurrent)) (.x (LocalVariables|GetLPosition))) (< (.y (LocalVariables|GetLCurrent)) (.y (LocalVariables|GetLPosition))))
          (LocalVariables|SetLPosition (LocalVariables|GetLCurrent))))
      (:NewEnumerator2
        (if (or (> (.x (LocalVariables|GetLCurrent)) (.x (LocalVariables|GetLPosition))) (> (.y (LocalVariables|GetLCurrent)) (.y (LocalVariables|GetLPosition))))
          (LocalVariables|SetLPosition (LocalVariables|GetLCurrent))))
      (:NewEnumerator3
        (if (or (< (.x (LocalVariables|GetLCurrent)) (.x (LocalVariables|GetLPosition))) (> (.y (LocalVariables|GetLCurrent)) (.y (LocalVariables|GetLPosition))))
          (LocalVariables|SetLPosition (LocalVariables|GetLCurrent))))))
  (return (LocalVariables|GetLPosition)))

(fn ModifyTextQuantity
  (bind _quantity (CallFunction|GetQuantity))
  (Rendering|Components|TextRender|SetText (Variables|Default|GetTextRender) (Utilities|Text|ToText(Integer) _quantity)))

(fn AdjustText
  (bind _gridsize (Utilities|GetClassDefaults "/Game/Inventory3D/Structure/BP_InventoryRule.BP_InventoryRule_C"))
  (Transformation|SetRelativeRotation (Variables|Default|GetTextRender) (Math|Rotator|MakeRotator 0.0 9e+01 (* (Variables|Default|GetCurrentRotation) -1.0)) false false)
  (bind _itemshape (CallFunction|GetItemShape))
  (bind _rotatedshape (Utilities|Rotate2DArray _itemshape (Variables|Default|GetCurrentRotation))
    (:%20%20
      (bind _return (Text|GetTextCoordinates _rotatedshape (Variables|Default|GetTextLocation)))
      (LocalVariables|SetLTextCoords _return)
      (bind (_xspan _yspan) (Utilities|GetMaxValues _rotatedshape)
        (:Completed
          (LocalVariables|SetLMaxX (- _xspan 1))
          (LocalVariables|SetLMaxY (- _yspan 1))
          (bind _output_get (LocalVariables|SetLTextCoords (|ModifyTextCoords)))
          (Transformation|SetRelativeLocation (Variables|Default|GetTextRender) (Math|Vector|MakeVector (.X (Math|Vector2D|BreakVector2D (- (* _output_get _gridsize) (* _gridsize -0.5)))) (.Y (Math|Vector2D|BreakVector2D (- (* _output_get _gridsize) (* _gridsize -0.5)))) (.z (Variables|/Script/Engine.SceneComponent|GetRelativeLocation (Variables|Default|GetTextRender)))) false false))))))

(fn AdjustRotation
  (bind _returnvalue (Utilities|GetUnitScaled))
  (Transformation|SetRelativeRotation (Variables|Default|GetStaticMesh) (Math|Rotator|MakeRotator 0.0 0.0 (Variables|Default|GetCurrentRotation)) false false)
  (bind _itemshape (CallFunction|GetItemShape))
  (bind _rotatedshape (Utilities|Rotate2DArray _itemshape (Variables|Default|GetCurrentRotation))
    (:%20%20
      (bind (_xspan _yspan) (Utilities|GetMaxValues _rotatedshape)
        (:Completed
          (Transformation|SetRelativeLocation (Variables|Default|GetStaticMesh) (* (Math|Vector|MakeVector (Math|Conversions|ToFloat(Integer) (* _yspan _returnvalue)) (Math|Conversions|ToFloat(Integer) (* _xspan _returnvalue -1.0)) 0.0) (|GetMultiplier)) false false))))))

(fn AdjustforGrabPoint
  (params (GrabPoint :type Vector%202D%20Structure))
  (bind _returnvalue (Utilities|GetUnitScaled))
  (bind _returnvalue_2 (+ GrabPoint "(X=0.500000,Y=0.500000)"))
  (bind _returnvalue_3 (* _returnvalue_2 _returnvalue))
  (bind (_x _y) (Math|Vector2D|BreakVector2D _returnvalue_3))
  (bind _returnvalue_4 (Math|Vector2D|MakeVector2D _y _x))
  (bind _returnvalue_5 (* _returnvalue_4 "(X=-1.000000,Y=1.000000)"))
  (Transformation|AddRelativeLocation (Variables|Default|GetStaticMesh) (Math|Vector|MakeVector (.x _returnvalue_5) (.y _returnvalue_5) (Math|Float|SelectFloat (Variables|Default|GetZOffset) 0.0 (Utilities|IsValid (Components|GetOwner)))) false false))

(fn AdjustTransformforWorld
  (Development|SetHiddeninGame (Variables|Default|GetTextRender) false false)
  (Transformation|SetActorScale3D "1.000000,1.000000,1.000000")
  (Transformation|SetRelativeScale3D (Variables|Default|GetStaticMesh) "1.000000,1.000000,1.000000"))

(fn AdjustTransformforGrid
  (Development|SetHiddeninGame (Variables|Default|GetTextRender) false false)
  (Transformation|SetRelativeRotation (Variables|Default|GetDefaultSceneRoot) "-90.000000,0.000000,0.000000" false false)
  (Transformation|SetRelativeScale3D (Variables|Default|GetStaticMesh) (Math|Conversions|ToVector(Float) (.InventoryScale (Utilities|GetClassDefaults "/Game/Inventory3D/Structure/BP_InventoryRule.BP_InventoryRule_C")))))

(fn AdjustLocation
  (bind _coordinates (CallFunction|GetCoordinates))
  (Transformation|SetActorRelativeLocation (Math|Vector|MakeVector 0.0 (.x (* _coordinates (Utilities|GetUnitScaled) "(X=-1.000000,Y=-1.000000)")) (.y (* _coordinates (Utilities|GetUnitScaled) "(X=-1.000000,Y=-1.000000)")))))

(fn ReceiveStartDragInventory
  (params (Handler :type AC%20Handler%20Object%20Reference) (DraggedItem :type Actor%20Object%20Reference) (GrabPoint :type Vector%202D%20Structure) (Coordinates :type Vector%202D%20Structure))
  (Transform|AdjustRotation)
  (Transform|AdjustforGrabPoint GrabPoint)
  (Text|AdjustText))

(fn ReceiveRotateItemInventory
  (params (Handler :type AC%20Handler%20Object%20Reference) (RotatedItem :type Actor%20Object%20Reference) (NewRotation :type Float%20%28double-precision%29) (GrabPoint :type Vector%202D%20Structure))
  (Variables|Default|SetCurrentRotation NewRotation)
  (Transform|AdjustRotation)
  (Transform|AdjustforGrabPoint GrabPoint)
  (Text|AdjustText))

(fn ReceiveDragExitInventory
  (params (Handler :type AC%20Handler%20Object%20Reference) (3D%20Inventory :type AC%203D%20Inventory%20Object%20Reference) (DraggedItem :type Actor%20Object%20Reference) (GrabPoint :type Vector%202D%20Structure))
  (Transform|AdjustRotation)
  (Transform|AdjustforGrabPoint GrabPoint))

(fn ReceiveDragEnterInventory
  (params (Handler :type AC%20Handler%20Object%20Reference) (3D%20Inventory :type AC%203D%20Inventory%20Object%20Reference) (DraggedItem :type Actor%20Object%20Reference) (GrabPoint :type Vector%202D%20Structure))
  (Transform|AdjustTransformforGrid)
  (Transform|AdjustRotation)
  (Transform|AdjustforGrabPoint GrabPoint)
  (Text|AdjustText))

(fn ReceiveEndDragWorld
  (params (Handler :type AC%20Handler%20Object%20Reference) (DroppedItem :type Actor%20Object%20Reference) (DropLocation :type Vector))
  (Class|BPIShareInfo|SetCoordinates(Message) self "(X=-1.000000,Y=-1.000000)")
  (Class|BPIShareInfo|SetRotation(Message) self 0.0))

(fn ReceiveStartDragWorld
  (params (Handler :type AC%20Handler%20Object%20Reference) (DraggedItem :type Actor%20Object%20Reference) (GrabPoint :type Vector%202D%20Structure) (WorldLocation :type Vector))
  (Transform|AdjustRotation)
  (Transform|AdjustforGrabPoint GrabPoint))

(fn ReceiveEndDragInventory
  (params (Handler :type AC%20Handler%20Object%20Reference) (3DInventory :type AC%203D%20Inventory%20Object%20Reference) (DroppedItem :type Actor%20Object%20Reference) (DroppedCoordinates :type Vector%202D%20Structure) (DroppedRotation :type Float%20%28double-precision%29))
  (if (!= (Components|GetOwner) 3DInventory)
    (Default|InventoryDisconnect Handler)
    (Transform|AdjustTransformforWorld)
    (Default|InventoryConnect Handler)
    (Transform|AdjustTransformforGrid))
  (Transform|AdjustLocation)
  (Transform|AdjustRotation)
  (Text|AdjustText))

(fn ReceiveMergeItemInventory
  (params (Handler :type AC%20Handler%20Object%20Reference) (DroppedItem :type Actor%20Object%20Reference) (Merged :type Array%20of%20Actor%20Object%20References) (OldQuantity :type Integer) (NewQuantity :type Integer)))

(fn ReceiveConsumedItemInventory
  (params (Handler :type AC%20Handler%20Object%20Reference) (3DInventory :type AC%203D%20Inventory%20Object%20Reference) (ConsumedItem :type Actor%20Object%20Reference))
  (Actor|DestroyActor ConsumedItem))

(fn ReceiveResetDragInventory
  (params (Handler :type AC%20Handler%20Object%20Reference) (3DInventory :type AC%203D%20Inventory%20Object%20Reference) (DroppedItem :type Actor%20Object%20Reference) (DroppedCoordinates :type Vector%202D%20Structure) (DroppedRotation :type Float%20%28double-precision%29))
  (if (!= (Components|GetOwner) 3DInventory)
    (Default|InventoryDisconnect Handler)
    (Transform|AdjustTransformforWorld)
    (Default|InventoryConnect Handler)
    (Transform|AdjustTransformforGrid))
  (bind _itemrotation (CallFunction|GetItemRotation))
  (Variables|Default|SetCurrentRotation _itemrotation)
  (Transform|AdjustLocation)
  (Transform|AdjustRotation)
  (Text|AdjustText))

(fn ReceiveResetDragWorld
  (params (Handler :type AC%20Handler%20Object%20Reference) (DroppedItem :type Actor%20Object%20Reference) (DropLocation :type Vector))
  (Transformation|SetActorLocation DropLocation false false)
  (Utilities|FlowControl|Sequence
    (:then_0
      (Development|SetHiddeninGame (Variables|Default|GetTextRender) true false)
      (Transformation|DetachFromActor self "KeepWorld" "KeepWorld" "KeepWorld")
      (Transformation|SetActorScale3D self "1.000000,1.000000,1.000000")
      (Transformation|SetRelativeScale3D (Variables|Default|GetStaticMesh) "1.000000,1.000000,1.000000")
      (Transformation|SetActorRotation "0, 0, 0")
      (Transform|AdjustRotation))
    (:then_1
      (Collision|SetActorEnableCollision true)
      (CallFunction|SetCoordinates "(X=-1.000000,Y=-1.000000)")
      (CallFunction|SetRotation 0.0))))

(fn GetCoordinates
  (return (Utilities|Struct|BreakST_InventoryItem (Variables|Default|GetItemData))))

(fn GetItemModel
  (return (Utilities|Struct|BreakST_InventoryItem (Variables|Default|GetItemData))))

(fn GetItemName
  (return (Utilities|Struct|BreakST_InventoryItem (Variables|Default|GetItemData))))

(fn GetItemRotation
  (return (Utilities|Struct|BreakST_InventoryItem (Variables|Default|GetItemData))))

(fn GetItemShape
  (return (Utilities|Struct|BreakST_InventoryItem (Variables|Default|GetItemData))))

(fn GetMaxQuantity
  (return (Utilities|Struct|BreakST_InventoryItem (Variables|Default|GetItemData))))

(fn GetObjectRef
  (return (Utilities|Struct|BreakST_InventoryItem (Variables|Default|GetItemData))))

(fn GetQuantity
  (return (Utilities|Struct|BreakST_InventoryItem (Variables|Default|GetItemData))))